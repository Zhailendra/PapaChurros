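; Player level system that tracks experience and levels up when the current threshold is reached.
; BeginPlay seeds the threshold from a base value, and AddExp accumulates experience, prints the total and calls LevelUp once it qualifies.
; LevelUp increments the level, resets experience to zero, discarding any overflow, and scales the next threshold linearly with level.
; An F2 key binding grants a fixed amount of experience, apparently for testing.
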(event EventBeginPlay
  (Variables|Default|SetTotalExpToNextLevel (Variables|Default|GetBaseExpNeededPerLevel)))

(event EventTick
  (params (DeltaSeconds :type Float%20%28single-precision%29)))

(event Input|KeyboardEvents|F2
  (params (Key :type Key%20Structure :default "None"))
  (:Pressed
    (CallFunction|AddExp 6)))

(fn AddExp
  (params (ExpGained :type Integer))
  (bind _output_get (Variables|Default|SetCurrentExp (+ ExpGained (Variables|Default|GetCurrentExp))))
  (Development|PrintText (Utilities|Text|ToText(Integer) _output_get))
  (if (>= (Variables|Default|GetCurrentExp) (Variables|Default|GetTotalExpToNextLevel))
    (CallFunction|LevelUp)))

(fn LevelUp
  (bind _result (Math|Integer|IncrementInt (Variables|Default|GetLevel))
    (:%20%20
      (Variables|Default|SetLevel _result)
      (Variables|Default|SetCurrentExp 0)
      (Variables|Default|SetTotalExpToNextLevel (* (Variables|Default|GetLevel) (Variables|Default|GetBaseExpNeededPerLevel))))))