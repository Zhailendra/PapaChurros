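; Player pawn for a food-service game where the player takes customer orders, works the fryer and drink station, and earns experience.
; Interactions branch on actor tags, switching between tagged fixed cameras and updating the gameplay widget.
; Taking an order registers it with the game instance and resets the drinker.
; Clicking that customer again scores food state and drink fill, adds experience, plays a happy or grumpy sound and destroys the customer.
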(event Custom|CompleteOrder
  (Variables|Default|SetisHappy true)
  (Variables|Default|SetRewardExp 0)
  (bind _returnvalue (Actor|GetActorOfClass "/Game/Blueprints/Tools/BP_Fryer.BP_Fryer_C"))
  (if (Utilities|Enum|Equal(Enum) (Variables|/Game/Blueprints/Food/BP_Churros.BP_Churros_C|GetState (.OutItem (Utilities|Array|Random (Variables|/Game/Blueprints/Tools/BP_Fryer.BP_Fryer_C|GetActorsInFryer _returnvalue)))) "NewEnumerator1")
    (Variables|Default|SetRewardExp (+ (Variables|Default|GetRewardExp) 3))
    (Variables|Default|SetisHappy true)
    (else
      (Variables|Default|SetRewardExp (+ (Variables|Default|GetRewardExp) 1))
      (Variables|Default|SetisHappy false)))
  (if (Variables|/Script/PapaChurros.BaseOrder|GetbHasDrink (Variables|/Script/PapaChurros.NpcActor|GetOrder (Variables|Default|GetCurrentCustomer)))
    (bind _returnvalue_2 (Actor|GetActorOfClass "/Game/Blueprints/Tools/BP_Drinker.BP_Drinker_C"))
    (Development|PrintText (Utilities|Text|ToText(Float) (Variables|/Game/Blueprints/Tools/BP_Drinker.BP_Drinker_C|GetPercentFull _returnvalue_2) "HalfToEven"))
    (if (and (>= (Variables|/Game/Blueprints/Tools/BP_Drinker.BP_Drinker_C|GetPercentFull _returnvalue_2) 0.6) (< (Variables|/Game/Blueprints/Tools/BP_Drinker.BP_Drinker_C|GetPercentFull _returnvalue_2) 0.8))
      (Variables|Default|SetRewardExp (+ (Variables|Default|GetRewardExp) 3))
      (Variables|Default|SetisHappy true)
      (else
        (Variables|Default|SetRewardExp (+ 1 (Variables|Default|GetRewardExp)))
        (Variables|Default|SetisHappy false))))
  (Default|AddExp (Variables|Default|GetBp_LevelSystem) (Variables|Default|GetRewardExp))
  (switch int (Math|Random|RandomInteger 2)
    (:0
      (if (Variables|Default|GetisHappy)
        (Audio|PlaySound2D "/Game/Resources/SFX/Happy01.Happy01" 1.0 1.0 0.0 0 0)
        (else
          (Audio|PlaySound2D "/Game/Resources/SFX/Grumpy01.Grumpy01" 1.0 1.0 0.0 0 0))))
    (:1
      (if (Variables|Default|GetisHappy)
        (Audio|PlaySound2D "/Game/Resources/SFX/Happy02.Happy02" 1.0 1.0 0.0 0 0)
        (else
          (Audio|PlaySound2D "/Game/Resources/SFX/Grumpy02.Grumpy02" 1.0 1.0 0.0 0 0))))
    (:2
      (if (Variables|Default|GetisHappy)
        (Audio|PlaySound2D "/Game/Resources/SFX/Happy03.Happy03" 1.0 1.0 0.0 0 0)
        (else
          (Audio|PlaySound2D "/Game/Resources/SFX/Grumpy03.Grumpy03" 1.0 1.0 0.0 0 0)))))
  (Actor|DestroyActor (Variables|Default|GetCurrentCustomer))
  (Variables|Default|SetCurrentCustomer 0))

(event EventInteractwithObject
  (params (InteractableActor :type Actor%20Object%20Reference))
  (bind _wb_gameplay (Variables|Default|GetWB_Gameplay))
  (bind _wb_gameplay_2 (Variables|Default|GetWB_Gameplay))
  (bind _wb_gameplay_3 (Variables|Default|GetWB_Gameplay))
  (if (Actor|ActorHasTag InteractableActor "LocalFryer")
    (Default|OpenTool _wb_gameplay_2)
    (Utilities|FlowControl|Delay 0.4)
    (CallFunction|BlendCamera "FryerCamera")
    (Variables|/Game/Blueprints/Widget/W_Gameplay.W_Gameplay_C|SetIsFriable _wb_gameplay_2 true)
    (Default|CallOrderStart)
    (elif (Actor|ActorHasTag InteractableActor "Customer")
      (Utilities|IsValid (Variables|Default|GetCurrentCustomer)
        (:Is%20Valid
          (if (== InteractableActor (Variables|Default|GetCurrentCustomer))
            (CallFunction|CompleteOrder)))
        (:Is%20Not%20Valid
          (bind _asbp_npc_actor (Utilities|Casting|CastToBP_NpcActor InteractableActor))
          (bind _output_get (Variables|Default|SetCurrentCustomer _asbp_npc_actor))
          (bind _asbp_base_game_instance (Utilities|Casting|CastToBP_BaseGameInstance (Game|GetGameInstance)))
          (Class|BaseGameInstance|AddOrder _asbp_base_game_instance (Class|NpcActor|GetOrder _output_get))
          (bind _returnvalue (Actor|GetActorOfClass "/Game/Blueprints/Tools/BP_Drinker.BP_Drinker_C"))
          (Default|ResetDrinker _returnvalue)
          (CallFunction|BlendCamera "BackCamera")
          (Default|OnDisplayOrders _wb_gameplay_3)
          (Utilities|Array|Clear (Variables|/Game/Blueprints/Widget/W_Gameplay.W_Gameplay_C|GetCompletedList _wb_gameplay_3))
          (Default|OnHideUpgrades _wb_gameplay_3)))
      (elif (Actor|ActorHasTag InteractableActor "LocalDrinker")
        (Default|OpenTool _wb_gameplay)
        (Utilities|FlowControl|Delay 0.4)
        (bind _returnvalue_2 (Actor|GetActorOfClass "/Game/Blueprints/Tools/BP_Drinker.BP_Drinker_C"))
        (Default|ResetDrinker _returnvalue_2)
        (CallFunction|BlendCamera "DrinkerCamera")
        (Variables|/Game/Blueprints/Widget/W_Gameplay.W_Gameplay_C|SetIsFriable _wb_gameplay false)))))

(event EventBeginPlay
  (bind _returnvalue (UserInterface|CreateWidget "/Game/Blueprints/Common/WBP_DebugInteract.WBP_DebugInteract_C"))
  (UserInterface|Viewport|AddtoViewport _returnvalue 0)
  (bind _returnvalue_2 (UserInterface|CreateWidget "/Game/Blueprints/Widget/W_Gameplay.W_Gameplay_C"))
  (bind _output_get (Variables|Default|SetWB_Gameplay _returnvalue_2))
  (UserInterface|Viewport|AddtoViewport _output_get 0)
  (Variables|/Game/Blueprints/Widget/W_Gameplay.W_Gameplay_C|SetPlayer _output_get self)
  (bind _outactors (Actor|GetAllActorswithTag "FrontCamera"))
  (Game|Player|SetViewTargetwithBlend (Game|GetPlayerController 0) (.OutItem (Utilities|Array|Random _outactors)) 0.0 "VTBlend_Linear" 0.0 false))

(fn ConstructionScript)

(fn BlendCamera
  (params (Camera :type String))
  (bind _outactors (Actor|GetAllActorswithTag (Utilities|String|StringToName Camera)))
  (Game|Player|SetViewTargetwithBlend (Game|GetPlayerController 0) (.OutItem (Utilities|Array|Random _outactors)) 0.0 "VTBlend_Linear" 0.0 false))