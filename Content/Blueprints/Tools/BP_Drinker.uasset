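; BP_Drinker is a touch-operated tool actor that moves a cup and fills its water while held.
; Touch begin and end call StartUse and EndUse, retrying until Cup is valid.
; A Timeline slides the cup to one of three scene points, randomly picked while the target still equals the start, and reverses on release.
; While in use, Tick raises the water's Z scale up to a clamp.
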(event Custom|EndUse
  (Variables|Default|SetIsInUse false)
  (bind _newtrack_0 (Timeline|Timeline Reverse)
    (:Update
      (Transformation|SetWorldLocation (Variables|Default|GetCup) (Math|Vector|Lerp(Vector) (Variables|Default|GetInitialPos) (Variables|Default|GetRandomPos) _newtrack_0) false false))))

(event Custom|StartUse
  (Variables|Default|SetIsInUse true)
  (if (Utilities|Operators|NotEqual(!=) (Variables|Default|GetRandomPos) (Variables|Default|GetInitialPos) 0.0)
    (bind _newtrack_0 (Timeline|Timeline Play)
      (:Update
        (Transformation|SetWorldLocation (Variables|Default|GetCup) (Math|Vector|Lerp(Vector) (Variables|Default|GetInitialPos) (Variables|Default|GetRandomPos) _newtrack_0) false false)))
    (else
      (CallFunction|SetRandomPos)
      (Timeline|Timeline Play))))

(event EventTick
  (params (DeltaSeconds :type Float%20%28single-precision%29))
  (bind _water (Variables|Default|GetWater))
  (bind _relativescale3d (Variables|/Script/Engine.SceneComponent|GetRelativeScale3D _water))
  (if (Variables|Default|GetIsInUse)
    (bind _output_get (Variables|Default|SetPercentFull (+ (Variables|Default|GetPercentFull) (* DeltaSeconds 0.2))))
    (Transformation|SetRelativeScale3D _water (Math|Vector|MakeVector (.x _relativescale3d) (.y _relativescale3d) (Math|Float|Clamp(Float) (Math|Float|Lerp 0.0 1e+01 _output_get) 0.0 7.0)))))

(event EventBeginPlay
  (bind _cup (Variables|Default|GetCup))
  (bind _points (Variables|Default|GetPoints))
  (bind _returnvalue (Transformation|GetWorldLocation _cup))
  (Utilities|Array|Add _points (Variables|Default|GetScene))
  (Utilities|Array|Add _points (Variables|Default|GetScene1))
  (Utilities|Array|Add _points (Variables|Default|GetScene2))
  (Variables|Default|SetInitialPos _returnvalue)
  (Variables|Default|SetRandomPos _returnvalue))

(event EventActorOnInputTouchBegin
  (params (FingerIndex :type ETouchIndex%20Enum :default "Touch1"))
  ;[1 1 1] Comment
  (Utilities|IsValid (Variables|Default|GetCup) :!label _label
    (:Is%20Valid
      (CallFunction|StartUse))
    (:Is%20Not%20Valid
      (Utilities|FlowControl|Delay 0.2)
      (goto _label))))

(event EventActorOnInputTouchEnd
  (params (FingerIndex :type ETouchIndex%20Enum :default "Touch1"))
  (Development|PrintString "end")
  (Utilities|IsValid (Variables|Default|GetCup) :!label _label
    (:Is%20Valid
      (CallFunction|EndUse))
    (:Is%20Not%20Valid
      (Utilities|FlowControl|Delay 0.2)
      (goto _label))))

(fn ConstructionScript)

(fn SetRandomPos
  (bind _points (Variables|Default|GetPoints))
  (Variables|Default|SetRandomPos (Transformation|GetWorldLocation (Utilities|Array|Get(acopy) _points (Math|Random|RandomIntegerinRange 0 (- (Utilities|Array|Length _points) 1))))))