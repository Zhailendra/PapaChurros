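; Fryer tool actor that moves its mesh between a raised and a resting position on touch and keeps a supply of churros.
; Touch begin and end wait for a valid ToolMesh, then a shared timeline lerps the mesh up or back down; release also mutes the oil sound.
; BeginPlay raises the mesh and spawns randomly rotated, scaled churros.
; Churros entering the Box are destroyed and respawned at the spawn point.
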(event OnComponentBeginOverlap(Box)
  (params (OverlappedComponent :type Primitive%20Component%20Object%20Reference) (OtherActor :type Actor%20Object%20Reference) (OtherComp :type Primitive%20Component%20Object%20Reference) (OtherBodyIndex :type Integer) (bFromSweep :type Boolean) (SweepResult :type Hit%20Result%20Structure%20%28by%20ref%29))
  (bind _asbp_churros (Utilities|Casting|CastToBP_Churros OtherActor))
  (Game|SpawnActorfromClass (Utilities|GetClass _asbp_churros) (Math|Transform|MakeTransform (.location (Transformation|GetWorldTransform (Variables|Default|GetChurrosSpawnPoint))) (Math|Random|RandomRotator false) (Math|Conversions|ToVector(Float) (Math|Random|RandomFloatinRange 0.7 1.0))) "Undefined" "MultiplyWithRoot" 0 0)
  (Actor|DestroyActor _asbp_churros))

(event EventTick
  (params (DeltaSeconds :type Float%20%28single-precision%29)))

(event EventActorOnInputTouchBegin
  (params (FingerIndex :type ETouchIndex%20Enum :default "Touch1"))
  ;[1 1 1] Comment
  (Utilities|IsValid (Variables|Default|GetToolMesh) :!label _label
    (:Is%20Valid
      (Class|Fryer|StartUse))
    (:Is%20Not%20Valid
      (Utilities|FlowControl|Delay 0.2)
      (goto _label))))

(event EventActorOnInputTouchEnd
  (params (FingerIndex :type ETouchIndex%20Enum :default "Touch1"))
  (Development|PrintString "end")
  (Utilities|IsValid (Variables|Default|GetToolMesh) :!label _label
    (:Is%20Valid
      (Class|Fryer|StopUse))
    (:Is%20Not%20Valid
      (Utilities|FlowControl|Delay 0.2)
      (goto _label))))

(event EventStartUse
  (Variables|Default|SetbIsInUse true)
  (Variables|Default|SetTime 0.0)
  (bind _newtrack_0 (Timeline|Timeline Reverse)
    (:Update
      (Transformation|SetWorldLocation (Variables|Default|GetFryerMesh) (Math|Vector|Lerp(Vector) (Variables|Default|GetFryerUpLocation) (Variables|Default|GetFryerDefaultLocation) _newtrack_0) false false))))

(event EventBeginPlay
  (bind _returnvalue (Transformation|GetActorLocation))
  (Audio|Components|Audio|SetVolumeMultiplier (Variables|Default|GetFryingOilIdleSound) 1.0 :!class /Script/Engine.AudioComponent)
  (Variables|Default|SetFryerDefaultLocation _returnvalue)
  (bind _output_get (Variables|Default|SetFryerUpLocation (+ _returnvalue "0.000000,0.000000,80.000000")))
  (Transformation|SetWorldLocation (Variables|Default|GetFryerMesh) _output_get false false)
  (for _index (range 0 (- (Variables|Default|GetChurrosNumber) 1))
    (Game|SpawnActorfromClass "/Game/Blueprints/Food/BP_Churros.BP_Churros_C" (Math|Transform|MakeTransform (.location (Transformation|GetWorldTransform (Variables|Default|GetChurrosSpawnPoint))) (Math|Random|RandomRotator false) (Math|Conversions|ToVector(Float) (Math|Random|RandomFloatinRange 0.7 1.0))) "AdjustIfPossibleButAlwaysSpawn" "MultiplyWithRoot" 0 0))
  (Development|PrintString "Churros Spawned"))

(event EventStopUse
  (Variables|Default|SetbIsInUse false)
  (Variables|Default|SetTime 0.0)
  (Audio|Components|Audio|SetVolumeMultiplier (Variables|Default|GetFryingOilIdleSound) 0.0 :!class /Script/Engine.AudioComponent)
  (bind _newtrack_0 (Timeline|Timeline Play)
    (:Update
      (Transformation|SetWorldLocation (Variables|Default|GetFryerMesh) (Math|Vector|Lerp(Vector) (Variables|Default|GetFryerUpLocation) (Variables|Default|GetFryerDefaultLocation) _newtrack_0) false false))))

(fn ConstructionScript)