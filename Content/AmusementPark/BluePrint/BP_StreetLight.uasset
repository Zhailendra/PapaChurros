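; BP_StreetLight is an amusement park street lamp with an optional decorative LED mesh, configured per instance in the editor.
; The construction script applies the exposed intensity (scaled by 100), radius, color and shadow settings to its point light.
; When the light is switched off, it zeroes and destroys the point light component, and a separate flag toggles the LED mesh's visibility.
; The event graph holds no runtime logic.
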(event EventBeginPlay)

(event Collision|EventActorBeginOverlap
  (params (OtherActor :type Actor%20Object%20Reference)))

(event EventTick
  (params (DeltaSeconds :type Float%20%28single-precision%29)))

(fn ConstructionScript
  (bind _pointlight (Variables|Default|GetPointLight))
  (bind _sm_streetled_02 (Variables|Default|GetSM_StreetLed_02))
  (bind _pointlight_2 (Variables|Default|GetPointLight))
  (if (Variables|Default|GetLightOn/Off)
    (Rendering|Components|Light|SetIntensity _pointlight_2 (* (Variables|Default|GetIntensity) 1e+02))
    (Rendering|Lighting|SetAttenuationRadius _pointlight_2 (Variables|Default|GetRadius))
    (Rendering|Components|Light|SetLightColor _pointlight_2 (Variables|Default|GetColor) true)
    (Rendering|Components|Light|SetCastShadows _pointlight_2 (Variables|Default|GetCastShadows?))
    (else
      (Rendering|Components|Light|SetIntensity _pointlight 0.0)
      (Rendering|Lighting|SetAttenuationRadius _pointlight 0.0)
      (Components|DestroyComponent _pointlight)))
  (if (Variables|Default|GetDecorativeLed?)
    (Rendering|SetVisibility _sm_streetled_02 true false)
    (else
      (Rendering|SetVisibility _sm_streetled_02 false false))))